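; BPC_Attacks is a character component that handles melee hit detection and damage.
; StartMeleeTrace starts a fast looping timer that sphere-traces between the supplied start and end objects' current world locations.
; A DoOnce passes only the first hit to the TakeDamage interface message, with the supplied DamageInfo and the owner as causer.
; StopMeleeTrace clears the timer and resets the DoOnce for the next attack.
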(event `Start Melee Trace`
  (params (`Trace Start Object` :type "SceneComponent Object Reference") (`Trace End Object` :type "SceneComponent Object Reference") (`Trace Radius` :type "Float (single-precision)") (DamageInfo :type "/Game/DamageSystem/S_DamageInfo Structure"))
  (bind _returnvalue (`KismetSystemLibrary.K2_SetTimerDelegate` (delegate `Melee Tarce`) 0.02 true))
  (set `self.Melee Trace Loop` _returnvalue))

(event `Melee Tarce`
  (bind (_outhit _returnvalue) (`KismetSystemLibrary.SphereTraceSingle` (`SceneComponent.K2_GetComponentLocation` (stale `Start Melee Trace` `Trace Start Object`)) (`SceneComponent.K2_GetComponentLocation` (stale `Start Melee Trace` `Trace End Object`)) (stale `Start Melee Trace` `Trace Radius`) "TraceTypeQuery3"))
  (if _returnvalue
    (`/Engine/EditorBlueprintResources/StandardMacros.DoOnce` false :!label _label
      (:`Completed`
        (message `/Game/DamageSystem/BPI_Damageable.TakeDamage` (`.HitActor` (`GameplayStatics.BreakHitResult` _outhit)) (stale `Start Melee Trace` DamageInfo) (`self.GetOwner`))))))

(event `StopMeleeTrace`
  (`KismetSystemLibrary.K2_ClearAndInvalidateTimerHandle` (`self.Melee Trace Loop`))
  (goto _label :!via `Reset`))