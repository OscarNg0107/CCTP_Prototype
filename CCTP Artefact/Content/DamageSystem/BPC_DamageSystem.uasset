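; BPC_DamageSystem is a damage component that tracks health, death and defensive states for its owner.
; TakeDamage uses CanBeDamaged to route each DamageInfo hit to block, damage or no damage, based on invincibility, death, parrying and blocking.
; Dispatchers report parries, blocks, death and damage responses, the last only when interruptible or forced.
; Heal restores clamped health while alive; TakeDamage returns whether damage landed.
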(fn `Heal`
  (params (`Heal Amount` :type "Float (double-precision)"))
  (returns (NewHealth :type "Float (double-precision)"))
  (if (not (`self.IsDead`))
    (bind _output_get (set `self.Health` (`KismetMathLibrary.FClamp` (+ (`self.Health`) `Heal Amount`) 0.0 (`self.MaxHealth`))))
    (return _output_get)))

(fn `TakeDamage`
  (params (DamageInfo :type "/Game/DamageSystem/S_DamageInfo Structure") (DamageCauser :type "Actor Object Reference"))
  (returns (WasDamaged :type Boolean))
  (bind (_damageamount _damagetype _damageresponse _shoulddamageinvincible _canbeblocked _canbeparried _shouldforceinterrupt) (break `/Game/DamageSystem/S_DamageInfo` DamageInfo))
  (bind _parry (`self.CanBeDamaged` _shoulddamageinvincible _canbeblocked _canbeparried)
    (:`BlockDamage`
      (if _parry
        (`self.OnParried` DamageCauser)
        (return false)
        (else
          (`self.OnBlocked` DamageCauser)
          (return false))))
    (:`DoDamage`
      (bind _output_get (set `self.Health` (- (`self.Health`) _damageamount)))
      (if (<= _output_get 0.0)
        (set `self.IsDead` true)
        (`self.OnDeath`)
        (elif (or (`self.IsInterruptible`) _shouldforceinterrupt)
          (`self.OnDamageResponse` _damageresponse DamageCauser)))
      (return true))
    (:`NoDamage`
      (return false))))